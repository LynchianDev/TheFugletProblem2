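; BP_FugletHand is a hand actor that lowers a Fuglet into the level and releases it as an AI pawn.
; Timelines lerp it down to a target height, where it swaps the child-actor Fuglet for a spawned BP_Fuglet_AI, then back up.
; At the top it destroys itself and its first attached actor, unless that is the player, which calls the empty EndGame event.
; An unused-here helper checks whether TargetFuglet is fully fed.
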(event `self.ReceiveBeginPlay`
  (bind _fuglet (`self.Fuglet`))
  (bind (_startlocation_x _startlocation_y) (`KismetMathLibrary.BreakVector` (`self.StartLocation`)))
  (bind (_returnvalue_location _returnvalue_rotation) (`KismetMathLibrary.BreakTransform` (`SceneComponent.K2_GetComponentToWorld` _fuglet)))
  (bind _asbp_fuglet_ai (cast `/Game/Fuglets/BP_Fuglet_AI` (`ChildActorComponent.ChildActor` (`self.Fuglet`))))
  (`CharacterMovementComponent.DisableMovement` (`Character.CharacterMovement` _asbp_fuglet_ai))
  (set `self.StartLocation` (`self.K2_GetActorLocation`))
  (bind (_direction _zmove) (`Timeline|MoveDown` :!via `PlayFromStart`)
    (:`Update`
      (`self.K2_SetActorLocation` (`KismetMathLibrary.VLerp` (`self.StartLocation`) (`KismetMathLibrary.MakeVector` _startlocation_x _startlocation_y (`self.TargetHeight`)) _zmove)))
    (:`Finished`
      (`AIBlueprintHelperLibrary.SpawnAIFromClass` "/Game/Fuglets/BP_Fuglet_AI.BP_Fuglet_AI_C" null _returnvalue_location _returnvalue_rotation true null)
      (`ActorComponent.K2_DestroyComponent` _fuglet)
      (`KismetSystemLibrary.Delay` 1.0)
      (`self.MoveUp`))))

(event `MoveUp`
  (set `self.CurrentLoc` (`self.K2_GetActorLocation`))
  (bind (_direction _zmove) (`Timeline|GoUp` :!via `PlayFromStart`)
    (:`Update`
      (`self.K2_SetActorLocation` (`KismetMathLibrary.VLerp` (`self.CurrentLoc`) (`self.StartLocation`) _zmove)))
    (:`Finished`
      (`self.DestroySelfAndHeldObject`))))

(event `End Game`)

(fn `DestroySelfAndHeldObject`
  (bind _output (`|GetArrayItem` (`self.GetAttachedActors` true)))
  (`/Engine/EditorBlueprintResources/StandardMacros.IsValid` _output
    (:`Is Valid`
      (cast `/Game/Fuglets/BP_Fuglet_Player` _output
        (:`then`
          (`self.End Game`))
        (:`CastFailed`
          (`self.K2_DestroyActor` _output)
          (`self.K2_DestroyActor` :!label _label))))
    (:`Is Not Valid`
      (goto _label))))

(fn `IsFugletFat?`
  (returns (TargetFuglet :type "/Game/Fuglets/BP_Fuglet Object Reference") (ReturnValue :type Boolean))
  (bind _targetfuglet (`self.TargetFuglet`))
  (return _targetfuglet (>= (`/Game/Fuglets/BP_Fuglet.FoodCount` _targetfuglet) (`/Game/Fuglets/BP_Fuglet.MaxFood` _targetfuglet))))

(fn `UserConstructionScript`)