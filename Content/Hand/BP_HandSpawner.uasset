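; BP_HandSpawner spawns hand actors at random points inside its box volume.
; On BeginPlay it starts a looping timer that spawns a BP_FeedingHand every SpawnInterval.
; A separate SpawnFugletHand event spawns a BP_FugletHand the same way, but nothing in this Blueprint calls it.
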(event `self.ReceiveBeginPlay`
  (`KismetSystemLibrary.K2_SetTimerDelegate` (delegate `SpawnHand`) (`self.SpawnInterval`) true))

(event `SpawnHand`
  (bind _box (`self.Box`))
  (`|SpawnActorFromClass` "/Game/Hand/BP_FeedingHand.BP_FeedingHand_C" (`KismetMathLibrary.MakeTransform` (`KismetMathLibrary.RandomPointInBoundingBox` (`SceneComponent.K2_GetComponentLocation` _box) (`BoxComponent.GetScaledBoxExtent` _box))) "Undefined" "OverrideRootScale" null null))

(event `SpawnFugletHand`
  (bind _box (`self.Box`))
  (`|SpawnActorFromClass` "/Game/Hand/BP_FugletHand.BP_FugletHand_C" (`KismetMathLibrary.MakeTransform` (`KismetMathLibrary.RandomPointInBoundingBox` (`SceneComponent.K2_GetComponentLocation` _box) (`BoxComponent.GetScaledBoxExtent` _box))) "Undefined" "OverrideRootScale" null null))

(fn `UserConstructionScript`)