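; Feeding hand actor that descends to a target height, waits, then rises back and removes itself along with what it holds, unless petting delays the retreat.
; When food is eaten it releases its grip via timeline, then uses Tick to follow the immobilized Fuglet while petting.
; A full Fuglet is attached and carried up while BP_HandSpawner spawns a Fuglet hand; otherwise it falls free.
; Carrying the player Fuglet away calls EndGame.
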(event `self.ReceiveBeginPlay`
  (bind (_startlocation_x _startlocation_y) (`KismetMathLibrary.BreakVector` (`self.StartLocation`)))
  (set `self.StartLocation` (`self.K2_GetActorLocation`))
  (bind (_direction _zmove) (`Timeline|MoveDown` :!via `PlayFromStart` :!label _label)
    (:`Update`
      (`self.K2_SetActorLocation` (`KismetMathLibrary.VLerp` (`self.StartLocation`) (`KismetMathLibrary.MakeVector` _startlocation_x _startlocation_y (`self.TargetHeight`)) _zmove)))
    (:`Finished`
      (`KismetSystemLibrary.Delay` 4.0)
      (if (not (`self.IsPetting`))
        (`self.MoveUp`)))))

(event `StopAllMovement`
  (`|ExecutionSequence`
    (:`then_0`
      (goto _label :!via `Stop`))
    (:`then_1`
      (bind (_direction _zmove) (`Timeline|GoUp` :!via `Stop` :!label _label_2)
        (:`Update`
          (`self.K2_SetActorLocation` (`KismetMathLibrary.VLerp` (`self.CurrentLoc`) (`self.StartLocation`) _zmove)))
        (:`Finished`
          (`self.DestroySelfAndHeldObject`))))))

(event `MoveUp`
  (set `self.CurrentLoc` (`self.K2_GetActorLocation`))
  (goto _label_2 :!via `PlayFromStart`))

(event `FoodEeaten`
  (params (EatingFuglet :type "/Game/Fuglets/BP_Fuglet Object Reference"))
  (bind (_targetfuglet _returnvalue) (`self.IsFugletFat?`))
  (set `self.TargetFuglet` EatingFuglet)
  (bind (_direction _newtrack_0) (`Timeline|ReleaseHand` :!via `PlayFromStart`)
    (:`Update`
      (set `self.GrabAmount` _newtrack_0))
    (:`Finished`
      (`/Engine/EditorBlueprintResources/StandardMacros.IsValid` (`self.TargetFuglet`)
        (:`Is Valid`
          (`self.SetActorTickEnabled` true)
          (`self.StopAllMovement`)
          (set `self.IsPetting` true)
          (`CharacterMovementComponent.DisableMovement` (`Character.CharacterMovement` (`self.TargetFuglet`)))
          (`KismetSystemLibrary.Delay` 2.5)
          (if _returnvalue
            (`self.K2_AttachToActor` (`self.TargetFuglet`) self "None" "KeepWorld" "KeepWorld" "KeepWorld" true)
            (bind _returnvalue_2 (`GameplayStatics.GetActorOfClass` "/Game/Hand/BP_HandSpawner.BP_HandSpawner_C"))
            (`/Game/Hand/BP_HandSpawner.SpawnFugletHand` _returnvalue_2)
            (else
              (`CharacterMovementComponent.SetMovementMode` (`Character.CharacterMovement` _targetfuglet) "MOVE_Falling" 0)))
          (set `self.IsPetting` false)
          (`self.SetActorTickEnabled` false)
          (`self.MoveUp`))))))

(event `self.ReceiveTick`
  (params (DeltaSeconds :type "Float (single-precision)"))
  (bind _targetfuglet (`self.TargetFuglet`)
    (:`then`
      (`SceneComponent.K2_SetWorldLocation` (`self.DefaultSceneRoot`) (`KismetMathLibrary.VInterpTo` (`self.K2_GetActorLocation`) (`self.K2_GetActorLocation` _targetfuglet) DeltaSeconds 8.0) false false))
    (:`else`)))

(fn `DestroySelfAndHeldObject`
  (bind _output (`|GetArrayItem` (`self.GetAttachedActors` true)))
  (`/Engine/EditorBlueprintResources/StandardMacros.IsValid` _output
    (:`Is Valid`
      (bind _asbp_fuglet_player (cast `/Game/Fuglets/BP_Fuglet_Player` _output)
        (:`then`
          (`/Game/Fuglets/BP_Fuglet_Player.EndGame` _asbp_fuglet_player))
        (:`CastFailed`
          (`self.K2_DestroyActor` _output)
          (`self.K2_DestroyActor` :!label _label))))
    (:`Is Not Valid`
      (goto _label))))

(fn `IsFugletFat?`
  (returns (TargetFuglet :type "/Game/Fuglets/BP_Fuglet Object Reference") (ReturnValue :type Boolean))
  (bind _targetfuglet (`self.TargetFuglet`)
    (:`then`
      (return _targetfuglet (>= (`/Game/Fuglets/BP_Fuglet.FoodCount` _targetfuglet) (`/Game/Fuglets/BP_Fuglet.MaxFood` _targetfuglet))))
    (:`else`)))

(fn `UserConstructionScript`)