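; BP_Kiddo is a character prop that periodically appears by moving vertically while its eyes follow BP_Fuglet_Player.
; After an initial delay, a looping Appear event plays a timeline that lerps Z between the start position and a fixed height, then waits a random interval.
; Appear enables Tick for the move, mapping player Y/Z to the EyePos parameter on a dynamic material instance created in the Construction Script.
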(event `self.ReceiveBeginPlay`
  (bind _returnvalue (`GameplayStatics.GetActorOfClass` "/Game/Fuglets/BP_Fuglet_Player.BP_Fuglet_Player_C"))
  (set `self.Player` _returnvalue)
  (set `self.StartPos` (`self.K2_GetActorLocation`))
  (`KismetSystemLibrary.Delay` 10.0)
  (`self.Appear`))

(event `Appear`
  (bind (_startpos_x _startpos_y _startpos_z) (`KismetMathLibrary.BreakVector` (`self.StartPos`)))
  (`self.SetActorTickEnabled` true)
  (bind (_direction _move) (`Timeline|Move`)
    (:`Update`
      (`self.K2_SetActorLocation` (`KismetMathLibrary.VLerp` (`KismetMathLibrary.MakeVector` _startpos_x _startpos_y _startpos_z) (`KismetMathLibrary.MakeVector` _startpos_x _startpos_y 330.0) _move)))
    (:`Finished`
      (`self.SetActorTickEnabled` false)
      (`KismetSystemLibrary.Delay` (`KismetMathLibrary.RandomFloatInRange` 10.0 20.0))
      (`self.Appear`))))

(event `self.ReceiveTick`
  (params (DeltaSeconds :type "Float (single-precision)"))
  (bind (_returnvalue_x _returnvalue_y _returnvalue_z) (`KismetMathLibrary.BreakVector` (`self.K2_GetActorLocation` (`self.Player`))))
  (`MaterialInstanceDynamic.SetVectorParameterValue` (`self.MatInst`) "EyePos" (make `LinearColor` (`KismetMathLibrary.MapRangeClamped` _returnvalue_y -1500.0 1500.0 -0.03 0.03) (`KismetMathLibrary.MapRangeClamped` _returnvalue_z 200.0 750.0 -0.03 0.03) 0.0 1.0)))

(fn `UserConstructionScript`
  (bind _returnvalue (`PrimitiveComponent.CreateDynamicMaterialInstance` (`self.StaticMeshComponent`) 0 "/Game/kiddo/kiddo_Mat.kiddo_Mat" "None"))
  (set `self.MatInst` _returnvalue))