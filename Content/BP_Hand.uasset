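; BP_Hand is a hand actor that moves to a target height, then returns to its spawn location and destroys itself.
; On BeginPlay, the MoveDown timeline lerps its Z to TargetHeight, and a fixed delay then triggers MoveUp.
; MoveUp can also interrupt the descent: it stops MoveDown and, guarded by a DoOnce, runs a second timeline from the current location back to the start.
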(event `self.ReceiveBeginPlay`
  (bind (_startlocation_x _startlocation_y) (`KismetMathLibrary.BreakVector` (`self.StartLocation`)))
  (set `self.StartLocation` (`self.K2_GetActorLocation`))
  (bind (_direction _zmove) (`Timeline|MoveDown` :!via `PlayFromStart` :!label _label)
    (:`Update`
      (`self.K2_SetActorLocation` (`KismetMathLibrary.VLerp` (`self.StartLocation`) (`KismetMathLibrary.MakeVector` _startlocation_x _startlocation_y (`self.TargetHeight`)) _zmove)))
    (:`Finished`
      (`KismetSystemLibrary.Delay` 4.0)
      (`self.MoveUp`))))

(event `MoveUp`
  (`|ExecutionSequence`
    (:`then_0`
      (goto _label :!via `Stop`))
    (:`then_1`
      (`/Engine/EditorBlueprintResources/StandardMacros.DoOnce` false
        (:`Completed`
          (set `self.CurrentLoc` (`self.K2_GetActorLocation`))
          (bind (_direction _zmove) (`Timeline|Timeline_0` :!via `PlayFromStart`)
            (:`Update`
              (`self.K2_SetActorLocation` (`KismetMathLibrary.VLerp` (`self.CurrentLoc`) (`self.StartLocation`) _zmove)))
            (:`Finished`
              (`self.K2_DestroyActor`))))))))

(fn `UserConstructionScript`)