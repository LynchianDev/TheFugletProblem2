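; BP_Shit is a bird-dropping actor (component Fugletshit) that animates its scale after spawning and varies in color.
; The construction script creates a dynamic material instance on that component and randomizes its RandomColor parameter.
; Tick eases the actor scale toward a tenth of its Size variable with VInterpTo.
; BeginPlay switches Tick off after a ten-second delay, leaving the actor static.
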(event `self.ReceiveBeginPlay`
  (`KismetSystemLibrary.Delay` 10.0)
  (`self.SetActorTickEnabled` false))

(event `self.ReceiveTick`
  (params (DeltaSeconds :type "Float (single-precision)"))
  (`self.SetActorScale3D` (`KismetMathLibrary.VInterpTo` (`self.GetActorScale3D`) (/ (`self.Size`) 10.0) DeltaSeconds 8.0)))

(fn `UserConstructionScript`
  (locals (MatInstance :type "MaterialInstanceDynamic Object Reference"))
  (bind _returnvalue (`PrimitiveComponent.CreateDynamicMaterialInstance` (`self.fugletshit`) 0 "/Game/Shit.Shit" "None"))
  (bind _output_get (set `local.MatInstance` _returnvalue))
  (`MaterialInstanceDynamic.SetScalarParameterValue` _output_get "RandomColor" (`KismetMathLibrary.RandomFloatInRange` -0.5 0.6)))