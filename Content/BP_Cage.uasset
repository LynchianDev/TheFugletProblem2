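; BP_Cage is a cage built from instanced meshes whose wood material reacts to how much the Fuglet player has eaten.
; The construction script rebuilds the hierarchical instanced static mesh from a Transforms array and gives it a dynamic instance of the Wood material.
; On BeginPlay it binds to the player's eat event, then sets the DeSaturate parameter to the ratio of FoodCount to MaxFood.
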(event `self.ReceiveBeginPlay`
  (bind _returnvalue (`GameplayStatics.GetActorOfClass` "/Game/Fuglets/BP_Fuglet_Player.BP_Fuglet_Player_C"))
  (bind _output_get (set `self.Player` _returnvalue))
  (add `/Game/Fuglets/BP_Fuglet_Player.PlayerEat` _output_get (delegate `AdjustMaterial`)))

(event `AdjustMaterial`
  (bind _player (`self.Player`))
  (`MaterialInstanceDynamic.SetScalarParameterValue` (`self.MatInst`) "DeSaturate" (/ (`KismetMathLibrary.Conv_IntToDouble` (`/Game/Fuglets/BP_Fuglet.FoodCount` _player)) (`KismetMathLibrary.Conv_IntToDouble` (`/Game/Fuglets/BP_Fuglet.MaxFood` _player)))))

(fn `UserConstructionScript`
  (`InstancedStaticMeshComponent.ClearInstances` (`self.HierarchicalInstancedStaticMesh`))
  (for _array_element (`self.Transforms`)
    (`InstancedStaticMeshComponent.AddInstance` (`self.HierarchicalInstancedStaticMesh`) _array_element))
  (bind _returnvalue (`PrimitiveComponent.CreateDynamicMaterialInstance` (`self.HierarchicalInstancedStaticMesh`) 0 "/Game/wood.wood" "None"))
  (set `self.MatInst` _returnvalue))